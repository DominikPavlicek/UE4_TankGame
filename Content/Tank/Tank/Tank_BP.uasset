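; Player-controllable tank Blueprint that wires input to its movement and aiming components.
; On BeginPlay it hands turret, barrel and both tracks to those components and sets itself as the health widget's tank reference.
; Movement axes pass intent to TankMovement, while aim axes rotate a separate azimuth gimbal and spring arm for the camera.
; Firing goes through TankAiming only in the Aimed state, with a 2D explosion sound.
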(event `self.ReceiveBeginPlay`
  (`TankAimingComponent.Initialise` (`self.TankAiming`) (`self.Tank Turret`) (`self.Tank Barrel`))
  (`TankMovementComponent.Initialise` (`self.TankMovement`) (`self.TankTracks_left`) (`self.TankTracks_right`))
  (`self.SetHealthBar`))

(event `InputAxis|Forward`
  (params (AxisValue :type "Float (single-precision)"))
  ;[1 1 1] Mvement
  (`TankMovementComponent.IntendMoveForward` (`self.TankMovement`) AxisValue))

(event `InputAxis|AimAzimuth`
  (params (AxisValue :type "Float (single-precision)"))
  ;[1 1 1] Camera
  ;;[1 1 1] On this Action
  ;;[1 1 1] Rotate the Spring Arm
  (`SceneComponent.K2_AddLocalRotation` (`self.AzimuthGimbal`) (`KismetMathLibrary.MakeRotator` 0.0 0.0 AxisValue) false false))

(event `InputAxis|MoveRigth`
  (params (AxisValue :type "Float (single-precision)"))
  ;[1 1 1] Mvement
  (`TankMovementComponent.IntendMoveRigth` (`self.TankMovement`) AxisValue))

(event `InputAxis|MoveLeft`
  (params (AxisValue :type "Float (single-precision)"))
  ;[1 1 1] Mvement
  (`TankMovementComponent.IntendMoveLeft` (`self.TankMovement`) AxisValue))

(event `InputAxis|AimElevation`
  (params (AxisValue :type "Float (single-precision)"))
  ;[1 1 1] Camera
  ;;[1 1 1] On this Action
  ;;[1 1 1] Rotate the Spring Arm
  (`SceneComponent.K2_AddLocalRotation` (`self.SpringArm`) (`KismetMathLibrary.MakeRotator` 0.0 AxisValue) false false))

(event `InputAction|FiringAction`
  (params (Key :type "Key Structure"))
  (bind _tankaiming (`self.TankAiming`))
  ;[1 1 1] Fire
  (:`Pressed`
    (switch `EFiringState` (`TankAimingComponent.GetFiringState` _tankaiming)
      (:`E_Ready`
        (`TankAimingComponent.Fire` _tankaiming)
        (`GameplayStatics.PlaySound2D` "/Game/StarterContent/Audio/Explosion01.Explosion01")))))

(fn `SetHealthBar`
  (bind _astank_hp (cast `/Game/HUD/TankHP` (`WidgetComponent.GetUserWidgetObject` (`self.Widget`)))
    (:`then`
      (set `/Game/HUD/TankHP.Tank Reference` self _astank_hp))
    (:`CastFailed`
      (`KismetSystemLibrary.PrintString` "TANK || Cast Tank HP to widget failed"))))

(fn `UserConstructionScript`)